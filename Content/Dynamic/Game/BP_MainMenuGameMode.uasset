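; Main menu game mode that plays an intro level sequence, then shows the main menu.
; BeginPlay creates a sequence player and starts it, and Tick polls until playback stops.
; A one-shot flag then guards creating the WP_MainMenu widget on the player screen and showing the mouse cursor.
; It sets UI-only input focused on the widget, then immediately overrides it with Game and UI mode using lock-on-capture.
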(event EventBeginPlay
  (bind _outactor (Sequencer|Player|CreateLevelSequencePlayer (Variables|Default|GetLevelSequence)))
  (bind _output_get (Variables|Default|SetSequenceActor _outactor))
  (Sequencer|Player|Play (Variables|/Script/LevelSequence.LevelSequenceActor|GetSequencePlayer _output_get) :!class /Script/MovieScene.MovieSceneSequencePlayer))

(event EventTick
  (params (DeltaSeconds :type Float%20%28single-precision%29))
  (bind _returnvalue (Game|GetPlayerController 0))
  (if (not (Variables|Default|GetOnlyOnce?))
    (if (not (Audio|Components|Audio|IsPlaying (Variables|/Script/LevelSequence.LevelSequenceActor|GetSequencePlayer (Variables|Default|GetSequenceActor))))
      (bind _returnvalue_2 (UserInterface|CreateWidget "/Game/Dynamic/UI/WP_MainMenu.WP_MainMenu_C" _returnvalue))
      (UserInterface|Viewport|AddtoPlayerScreen _returnvalue_2)
      (Variables|/Script/Engine.PlayerController|SetbShowMouseCursor _returnvalue true)
      (Input|SetInputModeUIOnly (Game|GetPlayerController 0) _returnvalue_2 "DoNotLock")
      (Variables|Default|SetOnlyOnce? true)
      (Input|SetInputModeGameandUI (Game|GetPlayerController 0) 0 "LockOnCapture" true))))

(fn ConstructionScript)