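; SpawnProjectiles is a splitting projectile actor that inherits its base behavior from a parent class.
; Shortly after BeginPlay, an original instance spawns three copies of its own class at random nearby offsets with the same rotation, then destroys itself.
; Each copy gets a projectile lifetime and an IsChild flag, set before its own delay ends, which stops it from splitting again.
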(event EventBeginPlay
  (|CallParentFunction)
  (Utilities|FlowControl|Delay 0.75)
  (if (not (Variables|Default|GetIsChild))
    (for _index (range 0 2)
      (bind _returnvalue (Game|SpawnActorfromClass "SpawnProjectiles_C" (Math|Transform|MakeTransform (+ (Transformation|GetActorLocation) (* (Math|Random|RandomUnitVector) 50)) (Transformation|GetActorRotation)) "AlwaysSpawn" 0 3.0 0))
      (Variables|SpawnProjectiles_C|SetIsChild _returnvalue true))
    (Actor|DestroyActor)))

(event Collision|EventActorBeginOverlap
  (params (OtherActor :type Actor%20Object%20Reference))
  (|CallParentFunction OtherActor) ; This node is disabled and will not be called.\nDrag off pins to build functionality.
)

(fn ConstructionScript
  (|CallParentFunction))