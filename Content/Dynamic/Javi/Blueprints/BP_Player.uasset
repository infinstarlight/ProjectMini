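; BP_Player is the player character, extending a parent character's weapon switching, attack, reload, death and dance events.
; It notifies the HUD of gun switches between normal, sticky, headshot and pushback, and disables walking movement during attacks and reloads until they finish.
; Shots are aimed from the shoot location toward the HUD's line-trace impact point, falling back to the trace direction.
; It also exposes health, ammo and name getters.
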(event EventBeginPlay
  (|CallParentFunction)
  (bind _asplayer_controller (Utilities|Casting|CastToPlayerController (Pawn|GetController))
    (:then
      (bind _output_get (Variables|MyGame|SetPC _asplayer_controller))
      (Variables|Default|SetHUD (HUD|GetHUD _output_get)))
    (:CastFailed
      (Development|PrintString "Need a player controller"))))

(event EventStartAttack
  (|CallParentFunction)
  (Pawn|Components|CharacterMovement|DisableMovement (Variables|Character|GetCharacterMovement)))

(event EventGetPushBack
  (Default|SpecialPowerPush (Variables|Default|GetPushBackGun) self))

(event EventStartReload
  (|CallParentFunction)
  (Pawn|Components|CharacterMovement|DisableMovement (Variables|Character|GetCharacterMovement)))

(event EventWeaponReload
  (|CallParentFunction)
  (Pawn|Components|CharacterMovement|SetMovementMode (Variables|Character|GetCharacterMovement) "MOVE_Walking" 0))

(event EventAddtoClipSize
  (params (AddToTotal :type Integer))
  (Default|AddtoMaxAmmo (Variables|Default|GetCurrentWeapon) AddToTotal))

(event EventGetStopAttack
  (Pawn|Components|CharacterMovement|SetMovementMode (Variables|Character|GetCharacterMovement) "MOVE_Walking" 0))

(event EventCharacterDeath
  (bind _pc (Variables|MyGame|GetPC))
  (|CallParentFunction)
  (Input|DisableInput _pc _pc)
  (Default|CallOnPlayerDeath)
  (Class|IHUD|DisableHUD(Message) (Variables|Default|GetHUD)))

(event EventStartSwitchSticky
  (|CallParentFunction)
  (Class|IHUD|GetStickyGun(Message) (Variables|Default|GetHUD)))

(event EventStartDance
  (|CallParentFunction)
  (Input|DisableInput (Game|GetPlayerController 0) 0))

(event EventStartSwitchWeapon
  (|CallParentFunction)
  (Class|IHUD|GetNormalGun(Message) (Variables|Default|GetHUD)))

(event EventStartSwitchHeadShot
  (|CallParentFunction)
  (Class|IHUD|GetHeadShotGun(Message) (Variables|Default|GetHUD)))

(event EventStartSwitchPushBack
  (|CallParentFunction)
  (Class|IHUD|GetPushBackGun(Message) (Variables|Default|GetHUD)))

(fn ConstructionScript
  (|CallParentFunction))

(fn GetShootTransform
  (bind (_result _direction _hitinfo) (Class|IHUD|GetLineTraceResults(Message) (Variables|Default|GetHUD)))
  (if _result
    (bind _location (CallFunction|GetShootLocation))
    (return (Math|Transform|MakeTransform _location (Math|Rotator|MakeRotfromX (- (.ImpactPoint (Collision|BreakHitResult _hitinfo)) _location))))
    (else
      (bind _location_2 (CallFunction|GetShootLocation))
      (return (Math|Transform|MakeTransform _location_2 _direction)))))

(fn GetAmmoRatio
  (bind _ratio (Default|AmmoRatio (Variables|Default|GetCurrentWeapon)))
  (return _ratio))

(fn GetHealthRatio
  (return (Default|GetRatio (Variables|Default|GetKillable))))

(fn GetPlayerName
  (return (Variables|MyGame|HUD|GetPlayerName)))