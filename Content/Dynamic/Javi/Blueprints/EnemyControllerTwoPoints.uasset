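; AI controller for the EnemyControllerTwoPoints enemy, which starts its behavior tree on BeginPlay.
; AI perception updates write a successfully sensed actor to the blackboard's player key and clear that key when sensing fails.
; The perception handler does not filter by actor type, so any sensed actor becomes the player value, and any lost stimulus clears it.
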(event OnTargetPerceptionUpdated(AIPerception)
  (params (Actor :type Actor%20Object%20Reference) (Stimulus :type AI%20Stimulus%20Structure))
  (if (.bSuccessfullySensed (Utilities|Struct|BreakAIStimulus Stimulus))
    (AI|Components|Blackboard|SetValueasObject (Variables|Default|GetBlackboard) (Variables|Default|GetPlayerKey) Actor)
    (else
      (AI|Components|Blackboard|ClearValue (Variables|Default|GetBlackboard) (Variables|Default|GetPlayerKey)))))

(event EventBeginPlay
  (AI|RunBehaviorTree (Variables|Default|GetBT)))

(event EventTick
  (params (DeltaSeconds :type Float%20%28single-precision%29)))

(fn ConstructionScript
  (|CallParentFunction))