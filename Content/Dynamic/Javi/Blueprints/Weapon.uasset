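; Weapon component for a pawn that fires projectiles from limited ammo, which fills to maximum on BeginPlay or reload.
; Shoot spends one round and spawns the projectile at a transform the owning pawn supplies through GetShootTransformMessage, with that pawn as instigator.
; Raising max ammo preserves the current fill ratio.
; SpecialPower is an empty function, while SpecialPowerPush applies a strong backward impulse to a given BP_Player.
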(event EventBeginPlay
  (CallFunction|Reload))

(fn Shoot
  (if (> (Variables|Default|GetCurrentAmmo) 0)
    (bind _aspawn (Utilities|Casting|CastToPawn (Components|GetOwner))
      (:then
        (bind _transform (Class|IUseWeapon|GetShootTransform(Message) _aspawn))
        (bind _returnvalue (Game|SpawnActorfromClass (Variables|Default|GetProjectileType) _transform "Undefined" 0 3.0 _aspawn))
        (Math|Integer|DecrementInt (Variables|Default|GetCurrentAmmo)
          (:%20%20
            (return _returnvalue))))
      (:CastFailed
        (Development|PrintString "Needs a pawn to have this component")
        (return 0)))
    (else
      (return 0))))

(fn Reload
  (Variables|Default|SetCurrentAmmo (Variables|Default|GetMaxAmmo)))

(fn AmmoRatio
  ;[1 1 1] Current / Max
  (return (/ (Math|Conversions|ToFloat(Integer) (Variables|Default|GetCurrentAmmo)) (Math|Conversions|ToFloat(Integer) (Variables|Default|GetMaxAmmo)))))

(fn AddtoMaxAmmo
  (params (AddedAmount :type Integer))
  (bind _ratio (CallFunction|AmmoRatio))
  (Variables|Default|SetMaxAmmo (+ AddedAmount (Variables|Default|GetMaxAmmo)))
  (Variables|Default|SetCurrentAmmo (Math|Float|Truncate (* (Variables|Default|GetMaxAmmo) _ratio))))

(fn SpecialPower)

(fn SpecialPowerPush
  (params (Actor :type Actor%20Object%20Reference))
  (bind _asbp_player (Utilities|Casting|CastToBP_Player Actor))
  (Physics|AddImpulse (Variables|/Script/Engine.Character|GetCharacterMovement _asbp_player) (* (Transformation|GetActorForwardVector Actor) -1.5e+04) true))

(fn GetCurrentAmmo
  (return (Variables|Default|GetCurrentAmmo)))