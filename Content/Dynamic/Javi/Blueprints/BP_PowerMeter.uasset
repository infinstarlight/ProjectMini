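; BP_PowerMeter is a clickable power meter actor that animates a value and lets the player lock it in.
; A timeline drives the UMG meter's fill and green-to-red color, along with a matching world text readout from 0 to 100.
; Clicks on its collision alternate via FlipFlop between stopping the timeline to store the value and flag it set, and resuming it to clear the flag.
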(event OnClicked(PowerMeterCollision)
  (params (TouchedComponent :type Primitive%20Component%20Object%20Reference) (ButtonPressed :type Key%20Structure))
  (Utilities|FlowControl|FlipFlop
    (:A
      (Audio|Components|Audio|Stop (Variables|Default|GetPower%20Meter%20Animation))
      (Variables|Default|SetPower%20Meter%20Value (Variables|/Game/MartinJavier/UMG/UMG_PowerMeter.UMG_PowerMeter_C|GetPower%20Meter%20Value (Variables|Default|GetPower%20Meter%20Reference)))
      (Variables|Default|SetbPower%20Value%20Set true))
    (:B
      (Audio|Components|Audio|Play (Variables|Default|GetPower%20Meter%20Animation))
      (Variables|Default|SetbPower%20Value%20Set false))))

(event Collision|EventActorBeginOverlap
  (params (OtherActor :type Actor%20Object%20Reference)))

(event EventBeginPlay
  (bind _asumg_power_meter (Utilities|Casting|CastToUMG_PowerMeter (UserInterface|GetUserWidgetObject (Variables|Default|GetUMG_PowerMeter))))
  (Variables|Default|SetPower%20Meter%20Reference _asumg_power_meter))

(event EventTick
  (params (DeltaSeconds :type Float%20%28single-precision%29)))

(fn ConstructionScript)