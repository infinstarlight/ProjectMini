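; Enemy is an AI-controlled character that extends a parent character class with weapon, reload, death and dance behavior.
; It mirrors the current weapon's ammo into the NumBullets blackboard key on begin play, attack and reload, and sends a ReloadComplete AI message after reloading.
; Death and dancing stop the behavior logic.
; When the death animation ends, it destroys itself and spawns an ammo clip-size pickup near its feet.
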(event EventBeginPlay
  (|CallParentFunction)
  (CallFunction|SetAmmoAI))

(event Collision|EventActorBeginOverlap
  (params (OtherActor :type Actor%20Object%20Reference)))

(event EventStartDance
  (AI|Logic|StopLogic (Variables|/Script/AIModule.AIController|GetBrainComponent (AI|GetAIController self)) "")
  (|CallParentFunction))

(event EventTick
  (params (DeltaSeconds :type Float%20%28single-precision%29)))

(event EventWeaponReload
  (|CallParentFunction)
  (CallFunction|SetAmmoAI)
  (Class|AIBlueprintHelperLibrary|SendAIMessage self "ReloadComplete" 0 true))

(event EventWeaponAttack
  (|CallParentFunction)
  (CallFunction|SetAmmoAI))

(event EventCharacterDeath
  (AI|Logic|StopLogic (Variables|/Script/AIModule.AIController|GetBrainComponent (AI|GetAIController self)) "")
  (|CallParentFunction))

(event EventDeathAnimEnded
  (Variables|Default|SetDeadEnemyLocation (Transformation|GetActorLocation))
  (Actor|DestroyActor)
  (Game|SpawnActorfromClass "/Game/MartinJavier/Blueprints/PickupAmmoClipSize.PickupAmmoClipSize_C" (Math|Conversions|ToTransform(Vector) (- (Variables|Default|GetDeadEnemyLocation) "0,0.000000,59.000000")) "Undefined" 0 0))

(fn ConstructionScript
  (|CallParentFunction))

(fn SetAmmoAI
  (Class|BlackboardComponent|SetValueasInt (AI|GetBlackboard (AI|GetAIController self)) (Utilities|Name|MakeLiteralName "NumBullets") (Default|GetCurrentAmmo (Variables|Default|GetCurrentWeapon))))