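; BP_GolfBall is a golf ball actor with a pickup collider and projectile movement, destroyed when picked up.
; An overlap on PickupCollider runs IsValidPickup, then OnPickup with the actor and hit, then AfterPickup, which destroys the ball.
; IsValidPickup accepts any actor and OnPickup is empty, so pickup itself has no other effect here.
; Unconnected leftover nodes for toggling collision and stopping the ball at near-zero speed never run.
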(event OnComponentBeginOverlap(PickupCollider)
  (params (OverlappedComponent :type Primitive%20Component%20Object%20Reference) (OtherActor :type Actor%20Object%20Reference) (OtherComp :type Primitive%20Component%20Object%20Reference) (OtherBodyIndex :type Integer) (bFromSweep :type Boolean) (SweepResult :type Hit%20Result%20Structure%20%28by%20ref%29))
  (bind _valid (CallFunction|IsValidPickup OtherActor))
  (if _valid
    (CallFunction|OnPickup OtherActor SweepResult)
    (CallFunction|AfterPickup)))

(event EventBeginPlay)

(event Collision|EventActorBeginOverlap
  (params (OtherActor :type Actor%20Object%20Reference)))

(event EventTick
  (params (DeltaSeconds :type Float%20%28single-precision%29)))

(fn ConstructionScript)

(fn IsValidPickup
  (params (Actor :type Actor%20Object%20Reference))
  (return true))

(fn OnPickup
  (params (Actor :type Actor%20Object%20Reference) (Hit%20Info :type Hit%20Result%20Structure)))

(fn AfterPickup
  (Actor|DestroyActor))