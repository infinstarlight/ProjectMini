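; HeadShotBullet is a projectile that only deals meaningful damage on headshots.
; On impact with a mesh component, it applies its full Damage if the hit bone is "head" and a token amount otherwise, then removes itself.
; Impacts on non-mesh components are ignored, with no damage and no removal call from this Blueprint.
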(event EventBeginPlay
  (|CallParentFunction) ; This node is disabled and will not be called.\nDrag off pins to build functionality.
)

(event Collision|EventActorBeginOverlap
  (params (OtherActor :type Actor%20Object%20Reference))
  (|CallParentFunction OtherActor) ; This node is disabled and will not be called.\nDrag off pins to build functionality.
)

(event EventOnImpact
  (params (DamagedActor :type Actor%20Object%20Reference) (HitInfo :type Hit%20Result%20Structure))
  (bind (_bblockinghit _binitialoverlap _time _distance _location _impactpoint _normal _impactnormal _physmat _hitactor _hitcomponent _hitbonename) (Collision|BreakHitResult HitInfo))
  (bind _returnvalue (Game|GetInstigatorController))
  (bind _self self)
  (Utilities|Casting|CastToMeshComponent _hitcomponent)
  (if (Utilities|Name|Equal(Name) _hitbonename "head")
    (Game|Damage|ApplyDamage DamagedActor (Variables|Default|GetDamage) _returnvalue _self "/Game/MartinJavier/Blueprints/DamageBase.DamageBase_C")
    (else
      (Game|Damage|ApplyDamage DamagedActor 0.1 _returnvalue _self "/Game/MartinJavier/Blueprints/DamageBase.DamageBase_C")))
  (CallFunction|RemoveProjectile))

(event EventTick
  (params (DeltaSeconds :type Float%20%28single-precision%29))
  (|CallParentFunction DeltaSeconds) ; This node is disabled and will not be called.\nDrag off pins to build functionality.
)

(fn ConstructionScript
  (|CallParentFunction))