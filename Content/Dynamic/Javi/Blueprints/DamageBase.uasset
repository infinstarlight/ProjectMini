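; DamageBase is a damage calculator that scales a base damage value by an elemental type: Fire, Ice or Lightning.
; GetDamage passes its inputs to CalculateFireDamage, which picks the ToFire, ToIce or ToLightning multiplier for that type and returns the product.
; Despite its name, CalculateFireDamage handles all three types.
; SpecialDamage takes an Actor but is a stub that always returns false.
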(fn CalculateFireDamage
  (params (BaseDamage :type Float%20%28single-precision%29) (Type :type E_Elements%20Enum :default "NewEnumerator0"))
  (switch Utilities|FlowControl|Switch|SwitchonE_Elements Type
    (:NewEnumerator0
      (LocalVariables|SetMultValue (Variables|Default|GetToFire)))
    (:NewEnumerator1
      (LocalVariables|SetMultValue (Variables|Default|GetToIce)))
    (:NewEnumerator2
      (LocalVariables|SetMultValue (Variables|Default|GetToLightning))))
  (return (* BaseDamage (LocalVariables|GetMultValue))))

(fn GetDamage
  (params (BaseDamage :type Float%20%28single-precision%29) (Type :type E_Elements%20Enum :default "NewEnumerator0"))
  (bind _realdamage (CallFunction|CalculateFireDamage BaseDamage Type))
  (return _realdamage))

(fn SpecialDamage
  (params (Actor :type Actor%20Object%20Reference))
  (return false))