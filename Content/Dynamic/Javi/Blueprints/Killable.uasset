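; Killable is an actor component that gives its owner health, reacts to the damage it takes, and signals hurt or death.
; It binds to the owner's OnTakeAnyDamage and, unless blocking, subtracts damage from clamped health, then calls OnHurt or OnDeath.
; Damage types implementing I_Damage adjust the amount using the component's element type and run a special effect message on non-lethal hits.
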(event Custom|TakeDamage
  (params (DamagedActor :type Actor%20Object%20Reference) (Damage :type Float%20%28single-precision%29) (DamageType :type Damage%20Type%20Object%20Reference) (InstigatedBy :type Controller%20Object%20Reference) (DamageCauser :type Actor%20Object%20Reference))
  (if (not (Variables|Default|GetBlock))
    (if (Utilities|DoesObjectImplementInterface DamageType "/Game/MartinJavier/Blueprints/I_Damage.I_Damage_C")
      (bind _realdamage (Class|IDamage|GetDamage(Message) DamageType Damage (Variables|Default|GetElementType)))
      (Utilities|Damaged _realdamage
        (:Hurt
          (Class|IDamage|SpecialDamage(Message) DamageType DamagedActor)
          (Default|CallOnHurt :!label _label))
        (:Dead
          (Default|CallOnDeath :!label _label_2)))
      (else
        (Utilities|Damaged Damage
          (:Hurt
            (goto _label))
          (:Dead
            (goto _label_2)))))))

(event EventBeginPlay
  (Variables|Default|SetCurrentHealth (Variables|Default|GetMaxHealth))
  (EventDispatchers|BindEventtoOnTakeAnyDamage (Components|GetOwner) (EventDispatchers|CreateEvent :!event Custom|TakeDamage)))

(fn GetRatio
  (return (/ (Variables|Default|GetCurrentHealth) (Variables|Default|GetMaxHealth))))

(fn RemoveHealth
  (params (InDamage :type Float%20%28single-precision%29))
  (bind _output_get (Variables|Default|SetCurrentHealth (Math|Float|Clamp(Float) (- (Variables|Default|GetCurrentHealth) InDamage) 0.0 (Variables|Default|GetMaxHealth))))
  (return _output_get))