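; StickyGun is a gun Blueprint whose special power detonates every live projectile it has fired.
; Shoot calls the parent implementation, stores each valid projectile in an array and binds to its destroyed event.
; RemoveProjectile takes destroyed projectiles out of that array.
; SpecialPower walks the array in reverse, calling Explode on each, which allows entries to be removed safely during the loop.
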(event EventBeginPlay
  (|CallParentFunction) ; This node is disabled and will not be called.\nDrag off pins to build functionality.
)

(event EventTick
  (params (DeltaSeconds :type Float%20%28single-precision%29)))

(event EventSpecialPower
  (bind _arrayelement (Utilities|Array|ReverseforEachLoop (Variables|Default|GetProjectiles))
    (:LoopBody
      (Default|Explode _arrayelement))))

(fn Shoot
  (bind _projectile (|CallParentFunction))
  (Utilities|IsValid _projectile
    (:Is%20Valid
      (Utilities|Array|Add (Variables|Default|GetProjectiles) _projectile)
      (Game|BindEventtoOnDestroyed _projectile (EventDispatchers|CreateEvent :!event RemoveProjectile))
      (return _projectile))))

(fn RemoveProjectile
  (params (Actor :type Actor%20Object%20Reference))
  (bind _asbase_projectile (Utilities|Casting|CastToBaseProjectile Actor)
    (:then
      (Utilities|Array|RemoveItem (Variables|Default|GetProjectiles) _asbase_projectile))
    (:CastFailed
      (Development|PrintString "This gun only shoots projectiles, what happened"))))