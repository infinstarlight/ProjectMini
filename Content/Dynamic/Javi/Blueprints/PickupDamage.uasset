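; PickupDamage is a pickup child Blueprint that deals continuous damage to an actor tagged "Base" while it stays in the pickup's collision.
; OnPickup stores the valid actor, and Tick applies frame-time-scaled damage to it using the DamagePopUp damage type.
; Ending any overlap on the collision clears the stored actor.
; AfterPickup is overridden with no behavior.
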(event OnComponentEndOverlap(Collision)
  (params (OverlappedComponent :type Primitive%20Component%20Object%20Reference) (OtherActor :type Actor%20Object%20Reference) (OtherComp :type Primitive%20Component%20Object%20Reference) (OtherBodyIndex :type Integer))
  (Variables|Default|SetActor 0))

(event EventTick
  (params (DeltaSeconds :type Float%20%28single-precision%29))
  (Game|Damage|ApplyDamage (Variables|Default|GetActor) DeltaSeconds 0 self "/Game/MartinJavier/Blueprints/DamagePopUp.DamagePopUp_C"))

(event EventOnPickup
  (params (Actor :type Actor%20Object%20Reference) (HitInfo :type Hit%20Result%20Structure))
  (Variables|Default|SetActor Actor))

(event EventAfterPickup)

(fn ConstructionScript
  (|CallParentFunction))

(fn IsValidPickup
  (params (Actor :type Actor%20Object%20Reference))
  (return (Actor|ActorHasTag Actor "Base")))