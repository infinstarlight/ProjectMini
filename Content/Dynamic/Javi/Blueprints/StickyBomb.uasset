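; StickyBomb is a projectile that sticks to what it hits and deals area damage when exploded.
; On impact with a mesh component, it disables collision, zeroes velocity and attaches at the hit bone, keeping world transform.
; Mesh and blocking impacts cancel the lifetime timer, so it waits for an Explode call not made here.
; Explode applies radial damage, draws a debug sphere, spawns a fire effect and removes the projectile.
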(event EventBeginPlay
  (|CallParentFunction) ; This node is disabled and will not be called.\nDrag off pins to build functionality.
)

(event Collision|EventActorBeginOverlap
  (params (OtherActor :type Actor%20Object%20Reference))
  (|CallParentFunction OtherActor) ; This node is disabled and will not be called.\nDrag off pins to build functionality.
)

(event EventTick
  (params (DeltaSeconds :type Float%20%28single-precision%29))
  (|CallParentFunction DeltaSeconds))

(event EventExplode
  (bind _returnvalue (Transformation|GetActorLocation))
  (Game|Damage|ApplyRadialDamage (Variables|Default|GetDamage) _returnvalue 5e+02 0 0 self (Game|GetInstigatorController) false "ECC_Visibility")
  (Rendering|Debug|DrawDebugSphere _returnvalue 5e+02 12 "(R=1.000000,G=0.299479,B=0.367504,A=1.000000)" 2.0 1.0)
  (Effects|SpawnEmitteratLocation "/Game/PGF2_Assets/VFX/P_Impact_Player_Fire_Strong.P_Impact_Player_Fire_Strong" _returnvalue "0, 0, 0" "8.000000,8.000000,8.000000")
  (CallFunction|RemoveProjectile))

(event EventOnImpact
  (params (DamagedActor :type Actor%20Object%20Reference) (HitInfo :type Hit%20Result%20Structure))
  (bind (_bblockinghit _binitialoverlap _time _distance _location _impactpoint _normal _impactnormal _physmat _hitactor _hitcomponent _hitbonename) (Collision|BreakHitResult HitInfo))
  (bind _asmesh_component (Utilities|Casting|CastToMeshComponent _hitcomponent))
  (Collision|SetActorEnableCollision false)
  (Variables|/Script/Engine.MovementComponent|SetVelocity (Variables|Default|GetProjectileMovement) "0, 0, 0")
  (Transformation|AttachComponentToComponent _asmesh_component _hitbonename "KeepWorld" "KeepWorld" "KeepWorld" true)
  (Utilities|Time|ClearandInvalidateTimerbyHandle (Variables|Default|GetLifeTimer)))

(event EventOnBlockingImpact
  (params (HitInfo :type Hit%20Result%20Structure))
  (Utilities|Time|ClearandInvalidateTimerbyHandle (Variables|Default|GetLifeTimer)))

(fn ConstructionScript
  (|CallParentFunction))