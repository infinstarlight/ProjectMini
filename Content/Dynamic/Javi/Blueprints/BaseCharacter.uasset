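; Base character Blueprint that provides a socketed extra mesh, a body tint function and placeholder hooks for animation, death and hurt handling.
; The construction script adds a skeletal mesh component and attaches it to the Gun socket of the character Mesh.
; SetBaseCharacterColor writes BodyColor on BaseMaterial, but the event graph logic that creates and applies that dynamic material is disconnected.
; SetAnimBP, CharacterDeath, CharacterHurt and BindKillableEvents are empty here.
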(fn ConstructionScript
  (bind _returnvalue (AddComponent|AddSkeletalMeshComponent false (Math|Transform|MakeTransform "0, 0, 0")))
  (Transformation|AttachComponentToComponent _returnvalue (Variables|Character|GetMesh) "Gun" "KeepRelative" "KeepRelative" "KeepRelative" true))

(fn SetAnimBP)

(fn CharacterDeath)

(fn CharacterHurt)

(fn BindKillableEvents)

(fn SetBaseCharacterColor
  (params (Color :type Linear%20Color%20Structure))
  (Rendering|Material|SetVectorParameterValue (Variables|Default|GetBaseMaterial) "BodyColor" Color :!class /Script/Engine.MaterialInstanceDynamic))