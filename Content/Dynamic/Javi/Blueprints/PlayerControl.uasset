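; Player controller that turns input into actions and movement on the controlled pawn.
; Action inputs for switching abilities or weapons, blocking, jumping, attacking, reloading and special power forward start messages to the pawn, with stop messages on releasing block and jump.
; MoveForward drives the pawn along its forward vector, with no strafe axis.
; Look axes feed yaw and pitch directly, while keyboard turning scales by TurnSpeed and delta time.
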(event Input|ActionEvents|InputActionAttack
  (params (Key :type Key%20Structure))
  (:Pressed
    (Class|ICharacter|StartAttack(Message) (Pawn|GetControlledPawn))))

(event Input|ActionEvents|InputActionReload
  (params (Key :type Key%20Structure))
  (:Pressed
    (Class|ICharacter|StartReload(Message) (Pawn|GetControlledPawn))))

(event Input|ActionEvents|InputActionJump
  (params (Key :type Key%20Structure))
  (bind _returnvalue (Pawn|GetControlledPawn))
  (:Pressed
    (Class|ICharacter|StartJump(Message) _returnvalue))
  (:Released
    (Class|ICharacter|StopJump(Message) _returnvalue)))

(event Input|ActionEvents|InputActionBlock
  (params (Key :type Key%20Structure))
  (bind _returnvalue (Pawn|GetControlledPawn))
  (:Pressed
    (Class|ICharacter|StartBlock(Message) _returnvalue))
  (:Released
    (Class|ICharacter|StopBlock(Message) _returnvalue)))

(event Input|ActionEvents|InputActionSpecialPower
  (params (Key :type Key%20Structure))
  (:Pressed
    (Class|ICharacter|StartSpecialPower(Message) (Pawn|GetControlledPawn))))

(event Input|ActionEvents|InputActionSwitchToPushBack
  (params (Key :type Key%20Structure))
  (:Pressed
    (Class|ICharacter|StartSwitchPushBack(Message) (Pawn|GetControlledPawn))))

(event Input|ActionEvents|InputActionSwitchToWeapon
  (params (Key :type Key%20Structure))
  (:Pressed
    (Class|ICharacter|StartSwitchWeapon(Message) (Pawn|GetControlledPawn))))

(event Input|ActionEvents|InputActionSWitchToSticky
  (params (Key :type Key%20Structure))
  (:Pressed
    (Class|ICharacter|StartSwitchSticky(Message) (Pawn|GetControlledPawn))))

(event Input|ActionEvents|InputActionSwitchToHeadShot
  (params (Key :type Key%20Structure))
  (:Pressed
    (Class|ICharacter|StartSwitchHeadShot(Message) (Pawn|GetControlledPawn))))

(event Input|ActionEvents|InputActionSwitchToSpawnProjectiles
  (params (Key :type Key%20Structure))
  (:Pressed
    (Class|ICharacter|StartSwitchSpawnProjectiles(Message) (Pawn|GetControlledPawn))))

(event Input|AxisEvents|InputAxisMoveForward
  (params (AxisValue :type Float%20%28single-precision%29))
  (bind _returnvalue (Pawn|GetControlledPawn))
  (Pawn|Input|AddMovementInput _returnvalue (Transformation|GetActorForwardVector _returnvalue) AxisValue false))

(event Input|AxisEvents|InputAxisLookRight
  (params (AxisValue :type Float%20%28single-precision%29))
  ;[1 1 1] Turning
  (Class|PlayerController|AddYawInput AxisValue))

(event Input|AxisEvents|InputAxisKB_Turn
  (params (AxisValue :type Float%20%28single-precision%29))
  ;[1 1 1] Turning
  (Class|PlayerController|AddYawInput (* AxisValue (Variables|Default|GetTurnSpeed) (Utilities|Time|GetWorldDeltaSeconds))))

(event Input|AxisEvents|InputAxisLookUp
  (params (AxisValue :type Float%20%28single-precision%29))
  ;[1 1 1] Turning
  (Class|PlayerController|AddPitchInput AxisValue))

(fn ConstructionScript)