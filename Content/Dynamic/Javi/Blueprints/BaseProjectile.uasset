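; Base projectile actor that damages what it overlaps and removes itself on impact or when its lifetime runs out.
; On spawn it applies its scale and starts a removal timer.
; Collision overlaps with damageable actors apply damage credited to the instigator, except the instigator itself, which routes to an empty self-impact hook.
; Blocking hits destroy it, and an empty Explode function is also defined.
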(event OnComponentBeginOverlap(Collision)
  (params (OverlappedComponent :type Primitive%20Component%20Object%20Reference) (OtherActor :type Actor%20Object%20Reference) (OtherComp :type Primitive%20Component%20Object%20Reference) (OtherBodyIndex :type Integer) (bFromSweep :type Boolean) (SweepResult :type Hit%20Result%20Structure%20%28by%20ref%29))
  (if (Variables|/Script/Engine.Actor|GetbCanBeDamaged OtherActor)
    (if (== (Game|GetInstigator) OtherActor)
      (CallFunction|OnSelfImpact SweepResult)
      (else
        (CallFunction|OnImpact OtherActor SweepResult)))))

(event OnComponentHit(Collision)
  (params (HitComponent :type Primitive%20Component%20Object%20Reference) (OtherActor :type Actor%20Object%20Reference) (OtherComp :type Primitive%20Component%20Object%20Reference) (NormalImpulse :type Vector :default "0, 0, 0") (Hit :type Hit%20Result%20Structure%20%28by%20ref%29))
  (CallFunction|OnBlockingImpact Hit))

(event Custom|RemoveProjectile
  (Actor|DestroyActor))

(event EventBeginPlay
  (Transformation|SetActorScale3D (Variables|Default|GetProjectileScale))
  (bind _returnvalue (Utilities|Time|SetTimerbyEvent (delegate Custom|RemoveProjectile) (Variables|Default|GetProjectile%20Life)))
  (Variables|Default|SetLifeTimer _returnvalue))

(event Collision|EventActorBeginOverlap
  (params (OtherActor :type Actor%20Object%20Reference)))

(event EventTick
  (params (DeltaSeconds :type Float%20%28single-precision%29)))

(fn ConstructionScript)

(fn OnImpact
  (params (DamagedActor :type Actor%20Object%20Reference) (HitInfo :type Hit%20Result%20Structure))
  (Game|Damage|ApplyDamage DamagedActor (Variables|Default|GetDamage) (Game|GetInstigatorController) self "/Game/MartinJavier/Blueprints/DamageBase.DamageBase_C")
  (CallFunction|RemoveProjectile))

(fn OnSelfImpact
  (params (HitInfo :type Hit%20Result%20Structure)))

(fn OnBlockingImpact
  (params (HitInfo :type Hit%20Result%20Structure))
  (CallFunction|RemoveProjectile))

(fn Explode)