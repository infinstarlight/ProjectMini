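; HipsCharacterWithGun is a character Blueprint that feeds aim rotation and crouch state to its Hips_Animation Anim Blueprint.
; On BeginPlay it casts the mesh's anim instance to Hips_Animation and caches it, printing a message if the cast fails.
; Each tick it writes the delta between control and actor rotation into the animation's TargetRotation.
; SetCrouched forwards the crouch flag to the animation.
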(event EventTick
  (params (DeltaSeconds :type Float%20%28single-precision%29))
  (Variables|/Game/PGF2_Assets/Levels/Blueprints/Hips_Animation.Hips_Animation_C|SetTargetRotation (Variables|Default|GetAnimBP) (Math|Rotator|Delta(Rotator) (Pawn|GetControlRotation :!class /Script/Engine.Pawn) (Transformation|GetActorRotation))))

(event EventBeginPlay
  (CallFunction|SetVaraibles))

(event EventSetCrouched
  (params (Crouch :type Boolean))
  (Variables|/Game/PGF2_Assets/Levels/Blueprints/Hips_Animation.Hips_Animation_C|SetCrouch (Variables|Default|GetAnimBP) Crouch))

(fn ConstructionScript)

(fn SetVaraibles
  (bind _aships_animation (Utilities|Casting|CastToHips_Animation (Components|SkeletalMesh|GetAnimInstance (Variables|Character|GetMesh)))
    (:then
      (Variables|Default|SetAnimBP _aships_animation))
    (:CastFailed
      (Development|PrintString "Theis needs the correct animation"))))