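; BP_Enemy is an enemy character that carries a weapon, takes damage and dies.
; On BeginPlay it spawns its weapon, attaches it to the mesh's pistol grip socket and caches the hero third-person animation Blueprint.
; Incoming damage goes to the AICharacterStats component, with current health printed as debug output.
; On death it sets the animation Blueprint's Dead flag and detaches from its controller.
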(event Game|Damage|EventAnyDamage
  (params (Damage :type Float%20%28single-precision%29) (DamageType :type Damage%20Type%20Object%20Reference) (InstigatedBy :type Controller%20Object%20Reference) (DamageCauser :type Actor%20Object%20Reference))
  (bind _aicharacterstats (Variables|Default|GetAICharacterStats))
  (Default|TakeDamage _aicharacterstats Damage)
  (Development|PrintString (Utilities|String|ToString(Float) (Variables|/Game/Dynamic/AI/AICharacterStats.AICharacterStats_C|GetCurrentHealth _aicharacterstats)))
  (if (Default|IsCharacterDead? _aicharacterstats)
    (Variables|/Game/Static/AnimStarterPack/UE4ASP_HeroTPP_AnimBlueprint.UE4ASP_HeroTPP_AnimBlueprint_C|SetDead? (Variables|Default|GetAnimBP) true)
    (Class|Pawn|DetachfromControllerPendingDestroy)))

(event EventBeginPlay
  (bind _returnvalue (Game|SpawnActorfromClass (Variables|Default|GetWeapon) (Math|Transform|MakeTransform "0, 0, 0") "Undefined" 0 0))
  (Variables|Default|SetWeaponEquipped _returnvalue)
  (Transformation|AttachComponentToComponent (Variables|/Script/Engine.Actor|GetRootComponent _returnvalue) (Variables|Character|GetMesh) "GripPoint_Pistol" "SnapToTarget" "SnapToTarget" "SnapToTarget" true)
  (bind _asue4asp_hero_tpp_anim_blueprint (Utilities|Casting|CastToUE4ASP_HeroTPP_AnimBlueprint (Components|SkeletalMesh|GetAnimInstance (Variables|Character|GetMesh))))
  (Variables|Default|SetAnimBP _asue4asp_hero_tpp_anim_blueprint))

(fn ConstructionScript)