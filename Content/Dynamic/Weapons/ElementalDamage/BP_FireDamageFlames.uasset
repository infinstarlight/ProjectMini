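; Fire damage flames actor that reacts when its box overlaps any actor other than player 0.
; It snaps its particle system onto the overlapped component and, if attachment succeeds, calls DestroyActor, then applies damage to that actor.
; A one-second retriggerable delay loops back to the attach step, but follows the destroy call.
; The lifespan-based destroy is disconnected and never runs.
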(event OnComponentBeginOverlap(Box)
  (params (OverlappedComponent :type Primitive%20Component%20Object%20Reference) (OtherActor :type Actor%20Object%20Reference) (OtherComp :type Primitive%20Component%20Object%20Reference) (OtherBodyIndex :type Integer) (bFromSweep :type Boolean) (SweepResult :type Hit%20Result%20Structure%20%28by%20ref%29))
  (if (not (== OtherActor (Game|GetPlayerCharacter 0)))
    (bind _returnvalue (Transformation|AttachComponentToComponent (Variables|Default|GetParticleSystem) OtherComp "None" "SnapToTarget" "SnapToTarget" "SnapToTarget" false :!label _label))
    (if _returnvalue
      (Actor|DestroyActor)
      (Game|Damage|ApplyDamage OtherActor (Variables|Default|GetDamage_0) (Game|GetInstigatorController) self "/Game/Dynamic/Weapons/DT_Base.DT_Base_C")
      (Utilities|FlowControl|Sequence
        (:then_0
          (Utilities|FlowControl|RetriggerableDelay 1.0)
          (goto _label))))))

(event EventBeginPlay)

(fn ConstructionScript)