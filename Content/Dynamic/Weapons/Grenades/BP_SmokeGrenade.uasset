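; BP_SmokeGrenade is a smoke grenade actor that creates a large smoke cloud after touching something other than the player character.
; Its sphere's begin-overlap event applies token damage to the overlapped actor, waits briefly, then spawns a scaled-up P_Smoke emitter at the grenade's location.
; The emitter's rotation is derived from the actor's location vector.
; The grenade destroys itself after a longer delay.
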(event OnComponentBeginOverlap(Sphere)
  (params (OverlappedComponent :type Primitive%20Component%20Object%20Reference) (OtherActor :type Actor%20Object%20Reference) (OtherComp :type Primitive%20Component%20Object%20Reference) (OtherBodyIndex :type Integer) (bFromSweep :type Boolean) (SweepResult :type Hit%20Result%20Structure%20%28by%20ref%29))
  (bind _returnvalue (Transformation|GetActorLocation))
  (if (not (== OtherActor (Game|GetPlayerCharacter 0)))
    (Game|Damage|ApplyDamage OtherActor 1.0 0 0)
    (Utilities|FlowControl|Delay 2.0)
    (Effects|SpawnEmitteratLocation "/Game/Static/StarterContent/Particles/P_Smoke.P_Smoke" _returnvalue (Math|Conversions|RotationFromXVector _returnvalue) "8.000000,8.000000,8.000000")
    (Utilities|FlowControl|Delay 6e+01)
    (Actor|DestroyActor)))

(event EventBeginPlay
  (|CallParentFunction) ; This node is disabled and will not be called.\nDrag off pins to build functionality.
)

(event Collision|EventActorBeginOverlap
  (params (OtherActor :type Actor%20Object%20Reference))
  (|CallParentFunction OtherActor) ; This node is disabled and will not be called.\nDrag off pins to build functionality.
)

(event EventTick
  (params (DeltaSeconds :type Float%20%28single-precision%29))
  (|CallParentFunction DeltaSeconds) ; This node is disabled and will not be called.\nDrag off pins to build functionality.
)

(fn ConstructionScript
  (|CallParentFunction))