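; Grenade actor that explodes on a timed fuse started when its sphere overlaps anything other than the player character.
; The overlap deals token contact damage, then a short delay precedes the explosion particles, sound and radial falloff damage.
; Blast damage comes from WeaponStats, is credited to the first player controller and can be blocked on the Vehicle channel.
; The actor then destroys itself and spawns a cracked-ground fire decal.
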(event OnComponentBeginOverlap(Sphere)
  (params (OverlappedComponent :type Primitive%20Component%20Object%20Reference) (OtherActor :type Actor%20Object%20Reference) (OtherComp :type Primitive%20Component%20Object%20Reference) (OtherBodyIndex :type Integer) (bFromSweep :type Boolean) (SweepResult :type Hit%20Result%20Structure%20%28by%20ref%29))
  (bind _returnvalue (Transformation|GetActorLocation))
  (if (not (== OtherActor (Game|GetPlayerCharacter 0)))
    (Game|Damage|ApplyDamage OtherActor 1.0 0 0)
    (Utilities|FlowControl|Delay 3.0)
    (Effects|SpawnEmitteratLocation "/Game/Static/StarterContent/Particles/P_Explosion.P_Explosion" _returnvalue (Math|Conversions|RotationFromXVector _returnvalue))
    (Class|GameplayStatics|ApplyRadialDamagewithFalloff (Variables|/Game/Dynamic/Weapons/WeaponStats.WeaponStats_C|GetDamageAmount (Variables|Default|GetWeaponStats)) 2.0 _returnvalue 1.5e+02 7.5e+02 2.0 0 0 self (Game|GetPlayerController 0) "ECC_Vehicle")
    (Audio|PlaySoundatLocation "/Game/Static/StarterContent/Audio/Explosion01.Explosion01" _returnvalue)
    (Actor|DestroyActor)
    (Rendering|Decal|SpawnDecalatLocation "/Game/InfinityBladeEffects/Effects/FX_Materials/Mobile/M_CrackedGround_Fire_Lit.M_CrackedGround_Fire_Lit" "1.000000,1.000000,1.000000" _returnvalue "0.000000,0.000000,0.000000" 0.0)))

(event EventBeginPlay
  (|CallParentFunction) ; This node is disabled and will not be called.\nDrag off pins to build functionality.
)

(event Collision|EventActorBeginOverlap
  (params (OtherActor :type Actor%20Object%20Reference))
  (|CallParentFunction OtherActor) ; This node is disabled and will not be called.\nDrag off pins to build functionality.
)

(event EventTick
  (params (DeltaSeconds :type Float%20%28single-precision%29))
  (|CallParentFunction DeltaSeconds) ; This node is disabled and will not be called.\nDrag off pins to build functionality.
)

(fn ConstructionScript
  (|CallParentFunction))