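; Player controller that handles a hard-coded local player join and opens the pause menu.
; Gamepad left face button checks whether the controller ID of player index 2 equals 2, and if so calls CreatePlayer for that index.
; The Pause action creates the WP_Pause widget, adds it to the viewport, shows the cursor and switches to UI-only input without pausing the game itself.
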(event EventBeginPlay)

(event EventTick
  (params (DeltaSeconds :type Float%20%28single-precision%29)))

(event Input|ActionEvents|InputActionPause
  (params (Key :type Key%20Structure))
  (:Pressed
    (bind _returnvalue (UserInterface|CreateWidget "/Game/Dynamic/UI/WP_Pause.WP_Pause_C" self))
    (UserInterface|Viewport|AddtoViewport _returnvalue 0)
    (Variables|Default|SetbShowMouseCursor true)
    (Input|SetInputModeUIOnly self _returnvalue "LockOnCapture")))

(event Input|GamepadEvents|GamepadFaceButtonLeft
  (params (Key :type Key%20Structure))
  (:Pressed
    (bind _returnvalue (Class|GameplayStatics|GetPlayerControllerID (Game|GetPlayerController 2)))
    (if (== _returnvalue 2)
      (Class|GameplayStatics|CreatePlayer 2))))

(fn ConstructionScript)