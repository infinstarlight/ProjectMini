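; Base Blueprint for AI-held weapons, providing hitscan firing, shot calculation and reloading.
; Fire spends ammo and traces from the player character's location to a point ahead of the weapon mesh, applying damage and playing sound only on a player hit.
; Calculate Shoot separately traces a spread cone from a camera, damages hits and returns a socket-based projectile transform and end point.
; Reload simply refills current ammo to maximum.
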(event EventBeginPlay)

(event Collision|EventActorBeginOverlap
  (params (OtherActor :type Actor%20Object%20Reference)))

(event EventTick
  (params (DeltaSeconds :type Float%20%28single-precision%29)))

(fn ConstructionScript)

(fn CalculateShoot
  (params (BaseDamage :type Float%20%28single-precision%29) (Camera :type Camera%20Component%20Object%20Reference) (WeaponMesh :type Scene%20Component%20Object%20Reference) (ProjectileSocket :type Name))
  (Utilities|FlowControl|Sequence
    (:then_0
      (LocalVariables|SetLocalCamera Camera)
      (LocalVariables|SetLocalWeaponMesh WeaponMesh)
      (LocalVariables|SetLocalWeaponSocket ProjectileSocket))
    (:then_1
      (LocalVariables|SetLocalEndLoc (+ (.location (Transformation|GetWorldTransform (LocalVariables|GetLocalCamera))) (* (Math|Random|RandomUnitVectorinConeinDegrees (Math|Vector|GetForwardVector (.rotation (Transformation|GetWorldTransform (LocalVariables|GetLocalCamera)))) (Variables|Default|GetSpreadCurrent)) 1e+04)))
      (bind (_outhit _returnvalue) (Collision|LineTraceForObjects (.location (Transformation|GetWorldTransform (LocalVariables|GetLocalCamera))) (+ (.location (Transformation|GetWorldTransform (LocalVariables|GetLocalCamera))) (* (Math|Random|RandomUnitVectorinConeinDegrees (Math|Vector|GetForwardVector (.rotation (Transformation|GetWorldTransform (LocalVariables|GetLocalCamera)))) (Variables|Default|GetSpreadCurrent)) 1e+04)) (Utilities|Array|MakeArray "ObjectTypeQuery1" "ObjectTypeQuery2" "ObjectTypeQuery3" "ObjectTypeQuery6") false 0 "ForDuration"))
      (if _returnvalue
        (LocalVariables|SetLocalTransfrom (Math|Transform|MakeTransform (Transformation|GetSocketLocation (Variables|Default|GetWeaponMesh) (LocalVariables|GetLocalWeaponSocket)) (Math|Rotator|FindLookatRotation (Transformation|GetSocketLocation (Variables|Default|GetWeaponMesh) (LocalVariables|GetLocalWeaponSocket)) (.ImpactPoint (Collision|BreakHitResult _outhit)))))
        (LocalVariables|SetLocalEndLoc (.ImpactPoint (Collision|BreakHitResult _outhit)))
        (if (.bBlockingHit (Collision|BreakHitResult _outhit))
          (Game|Damage|ApplyDamage (.HitActor (Collision|BreakHitResult _outhit)) BaseDamage 0 0))
        (else
          (LocalVariables|SetLocalTransfrom (Math|Transform|MakeTransform (Transformation|GetSocketLocation (Variables|Default|GetWeaponMesh) (LocalVariables|GetLocalWeaponSocket)) (Pawn|GetControlRotation (.AsPawn (Utilities|Casting|CastToPawn (Components|GetOwner (LocalVariables|GetLocalCamera)))) :!class /Script/Engine.Pawn))))))
    (:then_2
      (return (LocalVariables|GetLocalTransfrom) "" (LocalVariables|GetLocalEndLoc)))))

(fn Fire
  (bind _weaponmesh (Variables|Default|GetWeaponMesh))
  (bind _weaponstats (Variables|Default|GetWeaponStats))
  (bind _returnvalue (Transformation|GetWorldTransform _weaponmesh))
  (Variables|/Game/Dynamic/Weapons/WeaponStats.WeaponStats_C|SetCurrentAmmo _weaponstats (- (Variables|/Game/Dynamic/Weapons/WeaponStats.WeaponStats_C|GetCurrentAmmo _weaponstats) 1))
  (bind _outhit (Collision|LineTraceForObjects (Transformation|GetActorLocation (Game|GetPlayerCharacter 0)) (+ (.location _returnvalue) (* (Math|Random|RandomUnitVectorinConeinDegrees (Math|Vector|GetForwardVector (.rotation _returnvalue)) 0.0) 1.5e+04)) (Utilities|Array|MakeArray "ObjectTypeQuery3" "ObjectTypeQuery6") true 0 "None"))
  (if (.bBlockingHit (Collision|BreakHitResult _outhit))
    (if (== (.HitActor (Collision|BreakHitResult _outhit)) (Game|GetPlayerCharacter 0))
      (Game|Damage|ApplyDamage (.HitActor (Collision|BreakHitResult _outhit)) (Variables|/Game/Dynamic/Weapons/WeaponStats.WeaponStats_C|GetDamageAmount (Variables|Default|GetWeaponStats)) 0 0)
      (Audio|SpawnSoundatLocation (Variables|Default|GetWeaponFireSound) (.TraceStart (Collision|BreakHitResult _outhit))))))

(fn Reload
  (bind _weaponstats (Variables|Default|GetWeaponStats))
  (Variables|/Game/Dynamic/Weapons/WeaponStats.WeaponStats_C|SetCurrentAmmo _weaponstats (Variables|/Game/Dynamic/Weapons/WeaponStats.WeaponStats_C|GetMaxAmmo _weaponstats)))